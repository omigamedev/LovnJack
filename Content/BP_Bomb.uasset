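; Bomb actor that detonates once, either one second after BeginPlay or earlier when a BotChar overlaps its Cube.
; A shared DoOnce fires the RadialForce impulse and calls Explode on every BotChar within its radius, found by distance check.
; It then swaps components for effects and explosion audio, with an extra activation only for untouched timed blasts.
; A delayed fire sound follows on FuocoRestante regardless of trigger.
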(event OnComponentBeginOverlap(Cube)
  (params (OtherActor :type Actor%20Object%20Reference) (OtherComp :type Primitive%20Component%20Object%20Reference) (OtherBodyIndex :type Integer) (bFromSweep :type Boolean) (SweepResult :type Hit%20Result%20Structure%20%28by%20ref%29))
  (bind _radialforce (Variables|Default|GetRadialForce))
  (Utilities|Casting|CastToBotChar OtherActor)
  (Variables|Default|SetSpawnFire false)
  (Utilities|FlowControl|DoOnce false
    (:Completed
      (Class|RadialForceComponent|FireImpulse _radialforce)
      (bind _outactors (Actor|GetAllActorsOfClass "/Game/BotChar.BotChar_C"))
      (for _array_element _outactors
        (Math|Float|CompareFloat (Transformation|GetDistanceTo _array_element self) (Variables|/Script/Engine.RadialForceComponent|GetRadius _radialforce)
          (:<
            (Default|Explode _array_element))))
      (Components|DestroyComponent)
      (Components|Activation|Deactivate)
      (Components|Activation|Activate false)
      (if (Variables|Default|GetSpawnFire)
        (Components|Activation|Activate false))
      (Class|GameplayStatics|PlaySoundAttached "/Game/StarterContent/Audio/Explosion_Cue.Explosion_Cue" (Variables|Default|GetParticleSystem))
      (Utilities|FlowControl|Delay 1.0)
      (Class|GameplayStatics|PlaySoundAttached "/Game/StarterContent/Audio/Fire01_Cue.Fire01_Cue" (Variables|Default|GetFuocoRestante)))))

(event EventBeginPlay
  (bind _radialforce (Variables|Default|GetRadialForce))
  (Utilities|FlowControl|Delay 1.0)
  (Variables|Default|SetSpawnFire true)
  (Utilities|FlowControl|DoOnce false
    (:Completed
      (Class|RadialForceComponent|FireImpulse _radialforce)
      (bind _outactors (Actor|GetAllActorsOfClass "/Game/BotChar.BotChar_C"))
      (for _array_element _outactors
        (Math|Float|CompareFloat (Transformation|GetDistanceTo _array_element self) (Variables|/Script/Engine.RadialForceComponent|GetRadius _radialforce)
          (:<
            (Default|Explode _array_element))))
      (Components|DestroyComponent)
      (Components|Activation|Deactivate)
      (Components|Activation|Activate false)
      (if (Variables|Default|GetSpawnFire)
        (Components|Activation|Activate false))
      (Class|GameplayStatics|PlaySoundAttached "/Game/StarterContent/Audio/Explosion_Cue.Explosion_Cue" (Variables|Default|GetParticleSystem))
      (Utilities|FlowControl|Delay 1.0)
      (Class|GameplayStatics|PlaySoundAttached "/Game/StarterContent/Audio/Fire01_Cue.Fire01_Cue" (Variables|Default|GetFuocoRestante)))))

(fn ConstructionScript)